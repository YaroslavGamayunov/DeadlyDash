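; Enemy turret that turns its gun toward the player and fires projectiles, and is destroyed when the player touches its wire.
; The construction script builds the wire along a spline from spline meshes, with a box collision per section whose overlap triggers the explosion.
; Attack and AttackAborted play and reverse a charge timeline meant to update the charge widget and fire on completion.
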(event `self.ReceiveBeginPlay`
  (`|ExecutionSequence`
    (:`then_0`
      (for _array_element (`self.BoxCollisionsArray`)
        (add `PrimitiveComponent.OnComponentBeginOverlap` _array_element (delegate `WireOverlap`))))
    (:`then_1`
      (bind _aswb_turret_charge (cast `/Game/Main_Game/UI/WB_TurretCharge` (`WidgetComponent.GetWidget` (`self.Widget`))))
      (set `self.As WB Turret Charge` _aswb_turret_charge))))

(event `WireOverlap`
  (params (OverlappedComponent :type "PrimitiveComponent Object Reference") (OtherActor :type "Actor Object Reference") (OtherComp :type "PrimitiveComponent Object Reference") (OtherBodyIndex :type Integer) (bFromSweep :type Boolean) (SweepResult :type "HitResult Structure (by ref)"))
  (cast `/Game/Main_Game/Logic/A_Logic_Characters/Player/BP_PlayerCharacter` OtherActor)
  (`KismetSystemLibrary.PrintString` "TurretDeath")
  (`GameplayStatics.SpawnEmitterAtLocation` "/Game/Starter/StarterContent/Particles/P_Explosion.P_Explosion")
  (`self.K2_DestroyActor`))

(event `AttackAborted`
  (`TimelineComponent.Reverse` (`self.Charge_TL`)))

(event `Attack`
  (params (AttackTarget :type "Actor Object Reference"))
  (`TimelineComponent.Play` (`self.Charge_TL`)))

(event `self.ReceiveTick`
  (params (DeltaSeconds :type "Float (single-precision)"))
  (set `self.Delta Seconds` DeltaSeconds))

(event `Shoot`
  (bind _sphere (`self.Sphere`))
  (`|SpawnActorFromClass` "/Game/Main_Game/Logic/A_Logic_Characters/Projectiles/BP_Projectile_Runner.BP_Projectile_Runner_C" (`KismetMathLibrary.MakeTransform` (`SceneComponent.K2_GetComponentLocation` _sphere) (`KismetMathLibrary.Conv_VectorToRotator` (`SceneComponent.GetForwardVector` _sphere))) "AlwaysSpawn" "MultiplyWithRoot" null 1000.0 null)
  (`GameplayStatics.PlaySound2D` "/Engine/EditorSounds/GamePreview/EjectFromPlayer.EjectFromPlayer" 1.0 1.0 0.0 null null)
  (`self.AttackEnd`))

(event `self.TickEvent`
  (bind _gun (`self.Gun`))
  (`SceneComponent.K2_SetWorldRotation` (`self.Gun`) (`KismetMathLibrary.RInterpTo_Constant` (`SceneComponent.K2_GetComponentRotation` _gun) (`KismetMathLibrary.FindLookAtRotation` (`SceneComponent.K2_GetComponentLocation` _gun) (`self.K2_GetActorLocation` (`GameplayStatics.GetPlayerCharacter` 0))) (`self.Delta Seconds`) 300.0) false false))

(event `self.IdleEvent`
  (`GameplayStatics.SpawnEmitterAtLocation` "/Game/Starter/StarterContent/Particles/P_Explosion.P_Explosion" (`self.K2_GetActorLocation`)))

(fn `Get Position and Tangent`
  (params (LoopIndex :type Integer))
  (returns (Location :type "Vector Structure") (Tangent :type "Vector Structure"))
  (bind _spline (`self.Spline`))
  (bind _returnvalue (* LoopIndex (`self.SectionLength`)))
  (return (`SplineComponent.GetLocationAtDistanceAlongSpline` _spline _returnvalue "Local") (`KismetMathLibrary.ClampVectorSize` (`SplineComponent.GetTangentAtDistanceAlongSpline` _spline _returnvalue "Local") 0.0 (`self.SectionLength`))))

(fn `UserConstructionScript`
  (bind _returnvalue_x (`KismetMathLibrary.BreakVector` (`self.GetActorScale3D`)))
  (bind _returnvalue_location (`KismetMathLibrary.BreakTransform` (`SceneComponent.GetRelativeTransform` (`self.Spline`))))
  (set `self.SectionLength` (* _returnvalue_x 100.0))
  (bind _output_get (set `self.NumberOfSections` (`KismetMathLibrary.FTrunc` (/ (`SplineComponent.GetSplineLength` (`self.Spline`)) (`self.SectionLength`)))))
  (for _index (range (+ _output_get 1))
    (set `self.LoopIndex` _index)
    (bind _returnvalue (`AddComponent|NODE_AddSplineMeshComponent-0`))
    (`SplineMeshComponent.SetForwardAxis` _returnvalue "X" true)
    (bind (_location _tangent) (`self.Get Position and Tangent` (`self.LoopIndex`)))
    (bind (_location_2 _tangent_2) (`self.Get Position and Tangent` (+ (`self.LoopIndex`) 1)))
    (bind _returnvalue_2 (+ _returnvalue_location _location))
    (bind _returnvalue_3 (+ _location_2 _returnvalue_location))
    (`SplineMeshComponent.SetStartAndEnd` _returnvalue _returnvalue_2 _tangent _returnvalue_3 _tangent_2 true)
    (bind _returnvalue_4 (`AddComponent|NODE_AddBoxComponent-0` :`RelativeTransform` (`KismetMathLibrary.MakeTransform` (+ _returnvalue_2 (/ (- _returnvalue_3 _returnvalue_2) 2)) (`KismetMathLibrary.Conv_VectorToRotator` _tangent))))
    (`KismetArrayLibrary.Array_Add` (`self.BoxCollisionsArray`) _returnvalue_4)))