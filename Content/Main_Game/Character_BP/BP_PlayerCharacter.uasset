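; Player character Blueprint with two timeline-driven dashes, hit points and overlap damage to enemies, with death only printed.
; The semicircle dash follows a temporary spawned spline, invulnerable until finished.
; Line dash sets an offset target and plays BaseDashTL; the visible BaseDash_TL lerp movement and invulnerability reset are marked never run.
; Tick runs a vertical debug trace whose result is unused; test-widget creation is also unreached.
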(event `self.ReceiveBeginPlay`
  (`|ExecutionSequence`
    (:`then_0`
      (set `self.StartLocation` (`self.K2_GetActorLocation`))
      (set `PlayerController.bShowMouseCursor` true (`GameplayStatics.GetPlayerController` 0)))))

(event `SemiCircle_Dash`
  (params (`Spawn Transform Rotation` :type "Rotator Structure") (`Spawn Transform Scale` :type "Vector Structure"))
  (if (`TimelineComponent.IsPlaying` (`self.Timeline`))
    (`self.ReClick`))
  (set `self.bCanBeDamaged` false)
  (bind _returnvalue (`|SpawnActorFromClass` "/Game/Main_Game/Clicked_BP/SemiCircle_Spline.SemiCircle_Spline_C" (`KismetMathLibrary.MakeTransform` (`self.K2_GetActorLocation`) `Spawn Transform Rotation` `Spawn Transform Scale`) "Undefined" "MultiplyWithRoot" null null))
  (`TimelineComponent.SetPlayRate` (`self.Timeline`) (/ 1.0 (`self.Semi_Circle_Dash_Duration`)))
  (bind (_direction _newtrack_0) (`Timeline|Timeline` :!via `PlayFromStart`)
    (:`Update`
      (`self.K2_SetActorLocation` (`SplineComponent.GetLocationAtTime` (`/Game/Main_Game/Clicked_BP/SemiCircle_Spline.Spline` _returnvalue) _newtrack_0 "World" false)))
    (:`Finished`
      (set `self.StartLocation` (`self.K2_GetActorLocation`) :!label _label)
      (`KismetSystemLibrary.PrintString` "HADSSADASDllo")
      (`self.K2_DestroyActor` _returnvalue)
      (set `self.bCanBeDamaged` true))))

(event `ReClick`
  (goto _label))

(event `self.ReceiveAnyDamage`
  (params (Damage :type "Float (single-precision)") (DamageType :type "DamageType Object Reference") (InstigatedBy :type "Controller Object Reference") (DamageCauser :type "Actor Object Reference"))
  (bind _output_get (set `self.HitPoints` (- (`self.HitPoints`) Damage)))
  (if (<= _output_get 0.0)
    (`KismetSystemLibrary.PrintString` "DEATH")))

(event `Line_Dash`
  (params (DeltaLocation :type "Vector Structure"))
  (bind _basedash_tl (`self.BaseDash_TL`))
  (set `self.bCanBeDamaged` false)
  (set `self.FinalLocation` (+ (`self.StartLocation`) DeltaLocation))
  (`TimelineComponent.SetPlayRate` _basedash_tl (/ 1.0 (`self.Line_Dash_Duration`)))
  (`TimelineComponent.PlayFromStart` _basedash_tl))

(event `self.Box.OnComponentBeginOverlap`
  (params (OverlappedComponent :type "PrimitiveComponent Object Reference") (OtherActor :type "Actor Object Reference") (OtherComp :type "PrimitiveComponent Object Reference") (OtherBodyIndex :type Integer) (bFromSweep :type Boolean) (SweepResult :type "HitResult Structure (by ref)"))
  (bind _asbp_parent_enemy (cast `/Game/Main_Game/Enemy/BP_Parent_Enemy` OtherActor))
  (`GameplayStatics.ApplyDamage` _asbp_parent_enemy 1.0))

(event `self.ReceiveTick`
  (params (DeltaSeconds :type "Float (single-precision)"))
  (bind _returnvalue (`self.K2_GetActorLocation`))
  (`KismetSystemLibrary.LineTraceSingle` :`Start` (- _returnvalue (0.0 0.0 50.0)) :`End` (+ _returnvalue (0.0 0.0 50.0)) :`TraceChannel` "TraceTypeQuery1" :`DrawDebugType` "ForDuration"))

(fn `UserConstructionScript`)