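; Teleport wall that moves overlapping pawns to a facing surface along its Arrow direction, likely the opposite wall of the location.
; On Box overlap it line-traces a long fixed distance from the pawn for one custom object type, then targets a point just off the hit, along that actor's forward vector.
; The player character gets that point and a computed rotation through AfterTPAffectAnim, while other pawns are teleported directly with their rotation unchanged.
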(event `self.Box.OnComponentBeginOverlap`
  (params (OverlappedComponent :type "PrimitiveComponent Object Reference") (OtherActor :type "Actor Object Reference") (OtherComp :type "PrimitiveComponent Object Reference") (OtherBodyIndex :type Integer) (bFromSweep :type Boolean) (SweepResult :type "HitResult Structure (by ref)"))
  (bind _asbp_player_character (cast `/Game/Main_Game/A_Logic_Characters/Player/BP_PlayerCharacter` OtherActor)
    (:`then`
      (bind _returnvalue (`self.K2_GetActorLocation` _asbp_player_character))
      (bind (_outhit _returnvalue_2) (`KismetSystemLibrary.LineTraceSingleForObjects` _returnvalue (+ _returnvalue (* (`KismetMathLibrary.Normal` (`SceneComponent.GetForwardVector` (`self.Arrow`))) 10000.0)) (`|MakeArray` "ObjectTypeQuery7" :!type "EObjectTypeQuery Enum")))
      (if _returnvalue_2
        (bind (_bblockinghit _binitialoverlap _time _distance _location _impactpoint _normal _impactnormal _physmat _hitactor) (`GameplayStatics.BreakHitResult` _outhit))
        (bind _returnvalue_3 (`self.GetActorForwardVector` _hitactor))
        (bind _returnvalue_4 (* _returnvalue_3 100.0))
        (`/Game/Main_Game/A_Logic_Characters/Player/BP_PlayerCharacter.AfterTP_AffectAnim` _asbp_player_character (+ _impactpoint _returnvalue_4) (`KismetMathLibrary.FindLookAtRotation` _returnvalue_3 _returnvalue_4))))
    (:`CastFailed`
      (bind _aspawn (cast `Pawn` OtherActor))
      (bind _returnvalue_5 (`self.K2_GetActorLocation` _aspawn))
      (bind (_outhit_2 _returnvalue_6) (`KismetSystemLibrary.LineTraceSingleForObjects` _returnvalue_5 (+ _returnvalue_5 (* (`KismetMathLibrary.Normal` (`SceneComponent.GetForwardVector` (`self.Arrow`))) 10000.0)) (`|MakeArray` "ObjectTypeQuery7" :!type "EObjectTypeQuery Enum")))
      (if _returnvalue_6
        (bind (_bblockinghit_2 _binitialoverlap_2 _time_2 _distance_2 _location_2 _impactpoint_2 _normal_2 _impactnormal_2 _physmat_2 _hitactor_2) (`GameplayStatics.BreakHitResult` _outhit_2))
        (`self.K2_SetActorLocation` _aspawn (+ _impactpoint_2 (* (`self.GetActorForwardVector` _hitactor_2) 100.0)) false true)))))

(fn `UserConstructionScript`)