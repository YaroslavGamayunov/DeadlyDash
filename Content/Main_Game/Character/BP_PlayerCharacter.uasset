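; Player character Blueprint that handles spline-based dashing, damage and pausing.
; Dash spawns a spline actor and TextTrace and disables damage, with a timeline meant to move the character along the spline over DashDuration.
; AfterTP_AffectAnim teleports the character, restarts the dash and clears dash triggers, while ScreenCollision notifies triggers leaving the screen.
; Death, enemy-damage and debug trail logic is left disconnected.
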(event `self.ReceiveBeginPlay`
  (`|ExecutionSequence`
    (:`then_0`
      (set `self.FrameBackLocation` (`self.K2_GetActorLocation`)))))

(event `Dash`
  (params (`Spawn Transform Rotation` :type "Rotator Structure"))
  (bind _dash_tl (`self.Dash_TL`))
  (if (`TimelineComponent.IsPlaying` (`self.Dash_TL`))
    (`self.ReClick`))
  (set `self.bCanBeDamaged` false)
  (bind _returnvalue (`|SpawnActorFromClass` "/Game/Main_Game/A_Logic/Splines/BP_MainSpline_CharacterDash.BP_MainSpline_CharacterDash_C" (`KismetMathLibrary.MakeTransform` (`self.K2_GetActorLocation`) `Spawn Transform Rotation`) "Undefined" "MultiplyWithRoot" null null))
  (set `self.RelevantSplineActor` _returnvalue)
  (`TimelineComponent.SetPlayRate` _dash_tl (/ 1.0 (`self.Dash_Duration`)))
  (`TimelineComponent.PlayFromStart` _dash_tl)
  (bind _outactors (`GameplayStatics.GetAllActorsOfClass` "/Game/Main_Game/Character/TextTrace.TextTrace_C"))
  (for _array_element _outactors
    (`/Game/Main_Game/Character/TextTrace.stop` _array_element))
  (`|SpawnActorFromClass` "/Game/Main_Game/Character/TextTrace.TextTrace_C" (`KismetMathLibrary.MakeTransform` (0.0 0.0 0.0)) "AlwaysSpawn" "MultiplyWithRoot" null null))

(event `Pause`
  (`self.Pause_Menu_Ref` :!label _label
    (:`then`
      (bind _returnvalue (`|CreateWidget` "/Game/Main_Game/UI/Blueprints/WB_PauseMenu.WB_PauseMenu_C"))
      (bind _output_get (set `self.Pause_Menu_Ref` _returnvalue))
      (`UserWidget.AddToViewport` _output_get 0)
      (`GameplayStatics.SetGamePaused` true))
    (:`else`)))

(event `Key|Escape`
  (params (Key :type "Key Structure"))
  (:`Pressed`
    (goto _label)))

(event `self.ReceiveAnyDamage`
  (params (Damage :type "Float (single-precision)") (DamageType :type "DamageType Object Reference") (InstigatedBy :type "Controller Object Reference") (DamageCauser :type "Actor Object Reference"))
  (bind _output_get (set `self.HitPoints` (- (`self.HitPoints`) Damage)))
  (if (<= _output_get 0.0)
    _))

(event `Key|P`
  (params (Key :type "Key Structure"))
  (:`Pressed`
    (goto _label)))

(event `AfterTP_AffectAnim`
  (params (NewLocation :type "Vector Structure") (`Spawn Transform Rotation` :type "Rotator Structure"))
  (bind _dash_tl (`self.Dash_TL`))
  (`PrimitiveComponent.SetCollisionEnabled` (`self.ScreenCollision`) "NoCollision")
  (`TimelineComponent.Stop` (`self.Dash_TL`))
  (bind _relevantsplineactor (`self.RelevantSplineActor`)
    (:`then`
      (`self.K2_DestroyActor` _relevantsplineactor)
      (`self.K2_SetActorLocation` NewLocation false true)
      (bind _returnvalue (`|SpawnActorFromClass` "/Game/Main_Game/A_Logic/Splines/BP_MainSpline_CharacterDash.BP_MainSpline_CharacterDash_C" (`KismetMathLibrary.MakeTransform` (`self.K2_GetActorLocation`) `Spawn Transform Rotation`) "Undefined" "MultiplyWithRoot" null null))
      (set `self.RelevantSplineActor` _returnvalue)
      (`TimelineComponent.SetPlayRate` _dash_tl (/ 1.0 1.0))
      (`TimelineComponent.PlayFromStart` _dash_tl)
      (`KismetSystemLibrary.Delay` 0.5)
      (`/Game/Main_Game/Character/DashSpawner_Component.DestroyAllTriggers` (`self.DashSpawner_Component`))
      (`PrimitiveComponent.SetCollisionEnabled` (`self.ScreenCollision`) "QueryOnly"))
    (:`else`)))

(event `self.Box.OnComponentBeginOverlap`
  (params (OverlappedComponent :type "PrimitiveComponent Object Reference") (OtherActor :type "Actor Object Reference") (OtherComp :type "PrimitiveComponent Object Reference") (OtherBodyIndex :type Integer) (bFromSweep :type Boolean) (SweepResult :type "HitResult Structure (by ref)")))

(event `self.ScreenCollision.OnComponentEndOverlap`
  (params (OverlappedComponent :type "PrimitiveComponent Object Reference") (OtherActor :type "Actor Object Reference") (OtherComp :type "PrimitiveComponent Object Reference") (OtherBodyIndex :type Integer))
  (bind _asbp_dash_trigger (cast `/Game/Main_Game/A_Logic/BP_DashTrigger` OtherActor))
  (`/Game/Main_Game/A_Logic/BP_DashTrigger.LeftTheScreen` _asbp_dash_trigger))

(event `Trail`)

(event `ReClick`
  (`self.K2_DestroyActor` (`self.RelevantSplineActor`))
  (set `self.bCanBeDamaged` true))

(event `Timer Residual Trail`
  (set `self.stop trail` (`self.K2_GetActorLocation`))
  (bind _returnvalue (`KismetSystemLibrary.K2_SetTimerDelegate` (delegate `ResidualTrail`) 0.01 true))
  (set `self.NewVar` _returnvalue)
  (`KismetSystemLibrary.Delay` 5.0)
  (`KismetSystemLibrary.K2_ClearAndInvalidateTimerHandle` (`self.NewVar`)))

(event `ResidualTrail`
  (`KismetSystemLibrary.LineTraceSingle` :`Start` (`self.stop trail`) :`End` (`self.EndTrail`) :`TraceChannel` "TraceTypeQuery1" :`DrawDebugType` "ForDuration" :`TraceColor` (struct :`R` 0.081941 :`B` 1.0 :`A` 1.0) :`DrawTime` 0.0))

(fn `UserConstructionScript`)