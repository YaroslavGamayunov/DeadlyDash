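; BPC_DamageSystem is a damage system component that handles healing math and death detection.
; Heal returns current health plus the amount, clamped between zero and max health, without storing it.
; TakeDamage only checks whether incoming damage would deplete health, then flags death and calls OnDeath.
; Neither function writes current health, so non-lethal hits have no effect here.
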(fn `Heal`
  (params (Amount :type "Float (double-precision)"))
  (returns (NewHealth :type "Float (double-precision)"))
  (return (`KismetMathLibrary.FClamp` (+ Amount (`self.Health_Current`)) 0.0 (`self.Health_Max`))))

(fn `TakeDamage`
  (params (DamageInfo :type "/Game/Main_Game/Logic/DamageSystem/S_DamageInfo Structure"))
  (if (<= (- (`self.Health_Current`) (`.Amount_2_F6570A254EE22CA5365476B5707F34F3` (break `/Game/Main_Game/Logic/DamageSystem/S_DamageInfo` DamageInfo))) 0.0)
    (set `self.IsDead` true)
    (`self.OnDeath`)
    (return)))