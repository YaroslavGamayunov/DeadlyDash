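; Actor component that finds the interaction area under the mouse cursor and forwards interaction requests to its parent actor.
; Each Tick it line-traces on Visibility from the deprojected cursor to its projection on a Z plane.
; A new hit updates focus, toggling it on only for the exact BP_InteractionArea_CustomShape class.
; TryToInteract sends InteractMessage to the focused area's parent.
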(event `self.ReceiveTick`
  (params (DeltaSeconds :type "Float (single-precision)"))
  (`self.Trace`))

(event `TryToInteract`
  (params (In :type Boolean))
  (if (`self.IsTracingTheActor`)
    (message `/Game/Main_Game/Logic/Interfaces/Interactable_Interface.Interact` (`Actor.GetParentActor` (`self.Focused_Interaction Area`)))))

(fn `InteractionArea`
  (params (Trace :type Boolean))
  (if Trace
    (if (`self.IsTracingTheActor`)
      (`/Game/Main_Game/Logic/Interaction/InteractionArea/BP_InteractionArea_Master.ToggleFocus` (`self.Focused_Interaction Area`) false))
    (bind _asbp_interaction_area_master (cast `/Game/Main_Game/Logic/Interaction/InteractionArea/BP_InteractionArea_Master` (`self.FocusedActor`)))
    (bind _output_get (set `self.Focused_Interaction Area` _asbp_interaction_area_master))
    (`/Game/Main_Game/Logic/Interaction/InteractionArea/BP_InteractionArea_Master.ToggleFocus` _output_get true)
    (set `self.IsTracingTheActor` true)
    (elif (`self.IsTracingTheActor`)
      (bind _focused_interaction_area (`self.Focused_Interaction Area`)
        (:`then`
          (`/Game/Main_Game/Logic/Interaction/InteractionArea/BP_InteractionArea_Master.ToggleFocus` _focused_interaction_area false))
        (:`else`
          _))
      (set `self.IsTracingTheActor` false)
      (set `self.FocusedActor` null)
      (set `self.Focused_Interaction Area` null))))

(fn `Trace`
  (bind _focusedactor (`self.FocusedActor`))
  (bind (_outhit _returnvalue) (`KismetSystemLibrary.LineTraceSingle` (`PlayerController.DeprojectMousePositionToWorld` (`GameplayStatics.GetPlayerController` 0)) (`/Game/Main_Game/Logic/CoreUtils/BFL_NewNodes.Get Mouse projection on Z plane` (`self.Z Plane | Trace`)) "TraceTypeQuery1"))
  (if _returnvalue
    (bind (_bblockinghit _binitialoverlap _time _distance _location _impactpoint _normal _impactnormal _physmat _hitactor) (`GameplayStatics.BreakHitResult` _outhit))
    (if (!= _focusedactor _hitactor)
      (`self.FocusedActor`
        (:`then`
          (if (!= (`Actor.GetParentActor` _focusedactor) (`Actor.GetParentActor` _hitactor))
            (set `self.FocusedActor` _hitactor :!label _label)
            (`self.InteractionArea` (== (`GameplayStatics.GetObjectClass` _hitactor) "/Game/Main_Game/Logic/Interaction/InteractionArea/BP_InteractionArea_CustomShape.BP_InteractionArea_CustomShape_C"))))
        (:`else`
          (goto _label))))
    (else
      (`self.InteractionArea` false))))