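; Ability manager component on the player character that adds abilities as components and relays mouse events to them.
; AddAbility records the class, spawns any missing BPCA_Parent component and hands it the player reference.
; Each ability's info sorts it into hover-enter, hover-leave or click arrays, which transmitters bound to the interaction trace and player click call.
; RemoveAbility only destroys the passed component, leaving the arrays untouched.
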(event `self.ReceiveBeginPlay`
  (bind _asbp_player_character_parent (cast `/Game/Main_Game/Logic/A_Logic_Characters/Player/BP_PlayerCharacter_Parent` (`self.GetOwner`))
    (:`then`
      (set `self.As BP Player Character Parent` _asbp_player_character_parent))
    (:`CastFailed`
      (set `self.As BP Player Character Parent` null))))

(event `AddAbility`
  (params (NewItem :type "ActorComponent Class Reference (by ref)"))
  (`KismetArrayLibrary.Array_AddUnique` (`self.KnownAbilities`) NewItem)
  (`self.ActivateAddedAbilites`))

(event `RemoveAbility`
  (params (NewParam :type "ActorComponent Object Reference"))
  (`/Game/Main_Game/Logic/A_Logic_Characters/Player/BP_PlayerCharacter_Parent.DestroyComponent` (`self.As BP Player Character Parent`) NewParam))

(event `DebugTick`)

(event `ActivateAddedAbilites`
  (bind _returnvalue (`self.GetOwner`))
  (bind _ac_interactiontrace (`/Game/Main_Game/Logic/A_Logic_Characters/Player/BP_PlayerCharacter_Parent.AC_InteractionTrace` (`self.As BP Player Character Parent`)))
  (for _array_element (`self.KnownAbilities`)
    (`/Engine/EditorBlueprintResources/StandardMacros.IsValid` (`Actor.GetComponentByClass` _returnvalue _array_element)
      (:`Is Not Valid`
        (bind _returnvalue_2 (`|AddComponentByClass` _returnvalue _array_element))
        (bind _asbpca_parent (cast `/Game/Main_Game/Logic/Systems/Ability_System/AbilityEffects/BPCA_Parent` _returnvalue_2))
        (bind _output_get (set `self.As BPCA_P_Ref` _asbpca_parent))
        (set `/Game/Main_Game/Logic/Systems/Ability_System/AbilityEffects/BPCA_Parent.Player_Character` (`self.As BP Player Character Parent`) _output_get)
        (`KismetArrayLibrary.Array_AddUnique` (`self.CurrentAbilities`) _output_get))))
  ;[1 1 1] Comment
  (`self.AddedToApplyableArrays`)
  (add `/Game/Main_Game/Logic/Systems/Interaction_System/AC_InteractionTrace.OnMouseEnter` _ac_interactiontrace (delegate `OnMouseEnterTransmitter`))
  (add `/Game/Main_Game/Logic/Systems/Interaction_System/AC_InteractionTrace.OnMouseLeave` _ac_interactiontrace (delegate `OnMouseLeaveTransmitter`))
  (add `/Game/Main_Game/Logic/A_Logic_Characters/Player/BP_PlayerCharacter_Parent.OnClick` (`self.As BP Player Character Parent`) (delegate `OnMouseClickTransmitter`)))

(event `OnMouseLeaveTransmitter`
  ;[1 1 1] Comment
  (for _array_element (`self.Applyable_OnMouseLeave`)
    (`/Game/Main_Game/Logic/Systems/Ability_System/AbilityEffects/BPCA_Parent.OnMouseLeave_Effect` _array_element)))

(event `OnMouseClickTransmitter`
  ;[1 1 1] Comment
  (for _array_element (`self.Applyable_OnMouseClick`)
    (`/Game/Main_Game/Logic/Systems/Ability_System/AbilityEffects/BPCA_Parent.OnClickEffect` _array_element)))

(event `OnMouseEnterTransmitter`
  ;[1 1 1] Comment
  (for _array_element (`self.Applyable_OnMouseEnter`)
    (`/Game/Main_Game/Logic/Systems/Ability_System/AbilityEffects/BPCA_Parent.OnMouseEnter_Effect` _array_element)))

(fn `AddedToApplyableArrays`
  (for _array_element (`self.CurrentAbilities`)
    (bind _value (`/Game/Main_Game/Logic/Systems/Ability_System/AbilityEffects/BPCA_Parent.Get_AbilityInfo` _array_element (`GameplayStatics.GetObjectClass` _array_element)))
    (for _array_element_2 (`.AbilityApplyEvent_25_59582B6C4EE60C998B0B88B95D517C47` (break `/Game/Main_Game/Logic/Systems/Ability_System/DataAssets/S_AbilityData` _value))
      (`KismetArrayLibrary.Array_AddUnique` (select `/Game/Main_Game/Logic/Systems/Ability_System/DataAssets/E_AbilityApplyEvent` _array_element_2 :`NewEnumerator0` (`self.Applyable_OnMouseEnter`) :`NewEnumerator1` (`self.Applyable_OnMouseLeave`) :`NewEnumerator2` (`self.Applyable_OnMouseClick`)) _array_element))))