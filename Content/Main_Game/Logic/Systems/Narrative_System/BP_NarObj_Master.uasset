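; Master narrative object that shows a PDA note pop-up on focus and saves that note as known.
; Construction sets mesh and materials from the selected data table row, mirroring the mesh onto a dev-outlined spawn preview.
; BeginPlay picks a random unknown note matching scene and item, feeds it to PopUpComponent, and teleports the mesh to a random ScenePositions child.
; Focus changes toggle custom depth stencil and the pop-up.
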(event `self.ReceiveBeginPlay`
  (bind _popup_component (`self.PopUp_Component`))
  (bind _returnvalue (`KismetArrayLibrary.Array_Length` (`self.ValidNotes`)))
  (`|ExecutionSequence`
    (:`then_0`
      (for _array_element (`/Game/Main_Game/Logic/Systems/Narrative_System/PDA_Notes.All Notes_Array` (`self.PDA_Note`))
        (bind (_note_id _scene_id _pred_number _note_number _items) (break `/Game/Main_Game/Logic/Systems/Narrative_System/S_Note` _array_element))
        (if (== (`self.Scene_ID`) _scene_id)
          (if (== _items (`self.SelectName`))
            (bind _savednotes (message `/Game/Main_Game/Logic/SaveGame/BPI_SaveGame.GetKnownNotes` (`GameplayStatics.GetGameInstance`)))
            (if (== (`KismetArrayLibrary.Array_Find` _savednotes _array_element) -1)
              (`KismetArrayLibrary.Array_AddUnique` (`self.ValidNotes`) _array_element))))))
    (:`then_1`
      (if (!= _returnvalue 0)
        (bind _output_get (set `self.SelectedNote` (`|GetArrayItem` (`self.ValidNotes`) (`KismetMathLibrary.RandomInteger` _returnvalue))))
        (bind (_note_id_2 _scene_id_2 _pred_number_2 _note_number_2 _items_2 _az_type _text) (break `/Game/Main_Game/Logic/Systems/Narrative_System/S_Note` _output_get))
        (set `/Game/Main_Game/Logic/PopUp_Component.Text Pop Up` _text _popup_component)
        (set `/Game/Main_Game/Logic/PopUp_Component.Pred Number` _pred_number_2 _popup_component)
        (set `/Game/Main_Game/Logic/PopUp_Component.Note Number` _note_number_2 _popup_component)))
    (:`then_2`
      (for _array_element_2 (`SceneComponent.GetChildrenComponents` (`self.ScenePositions`) false)
        (`KismetArrayLibrary.Array_AddUnique` (`self.ListLocationsToSpawn`) (`SceneComponent.K2_GetComponentToWorld` _array_element_2)))
      (`SceneComponent.K2_SetWorldTransform` (`self.StaticMesh`) (`KismetArrayLibrary.Array_Random` (`self.ListLocationsToSpawn`)) false true))))

(event `OnMouseEnter`
  (`/Game/Main_Game/Logic/PopUp_Component.ShowPopUp` (`self.PopUp_Component`))
  (message `/Game/Main_Game/Logic/SaveGame/BPI_SaveGame.SaveKnownNotes_Data` (`GameplayStatics.GetGameInstance`) (`self.SelectedNote`) true))

(event `OnMouseLeave`
  (`/Game/Main_Game/Logic/PopUp_Component.RemovePopUp` (`self.PopUp_Component`)))

(fn `Interact`
  (params (`Actor Causer` :type "Actor Object Reference"))
  (returns (Success :type Boolean))
  (return false))

(fn `Interact_ToggleFocus_T`
  (params (Focus :type Boolean))
  (returns (SubjectToAbility :type Boolean))
  (if Focus
    (`PrimitiveComponent.SetCustomDepthStencilValue` (`self.StaticMesh`) 0)
    (`self.OnMouseEnter`)
    (else
      (`PrimitiveComponent.SetCustomDepthStencilValue` (`self.StaticMesh`) 4)
      (`self.OnMouseLeave`)))
  (return (`self.Subject to Ability`)))

(fn `UserConstructionScript`
  (`KismetArrayLibrary.Array_Clear` (`self.ValidNotes`))
  (bind _outrownames (`DataTableFunctionLibrary.GetDataTableRowNames` (`self.Data`)))
  (set `self.OptionsNames` _outrownames)
  (bind _returnvalue (`|GetDataTableRow` (`self.Data`) (`self.SelectName`))
    (:`then`
      (set `self.StructItem` _returnvalue)
      (`|ExecutionSequence`
        (:`then_0`
          (bind (_mesh _material_inst) (break `/Game/Main_Game/Logic/Data/Notes/Struct_ItemNotes` _returnvalue))
          (`StaticMeshComponent.SetStaticMesh` (`self.StaticMesh`) _mesh)
          (for _array_element (`PrimitiveComponent.GetMaterialSlotNames` (`self.StaticMesh`))
            (`PrimitiveComponent.SetMaterialByName` (`self.StaticMesh`) _array_element _material_inst)))
        (:`then_1`
          (`StaticMeshComponent.SetStaticMesh` (`self.SpawnPositionMesh`) _mesh)
          (for _array_element_2 (`PrimitiveComponent.GetMaterialSlotNames` (`self.SpawnPositionMesh`))
            (`PrimitiveComponent.SetMaterialByName` (`self.SpawnPositionMesh`) _array_element_2 "/Game/Main_Game/Logic/Systems/Interaction_System/InteractionArea/M_DEV_Outline.M_DEV_Outline")))))))