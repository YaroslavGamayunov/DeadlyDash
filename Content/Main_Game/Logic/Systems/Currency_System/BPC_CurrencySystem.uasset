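; BPC_CurrencySystem is a currency component that holds a single Currency balance for the game.
; AddCurrency increases the balance by a given amount and returns the new total.
; SubtractCurrency deducts an amount, clamps the balance at zero and returns it, with no signal when funds are insufficient.
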(fn `AddCurrency`
  (params (Amount :type "Float (double-precision)"))
  (returns (NewCurrency :type "Float (double-precision)"))
  (bind _output_get (set `self.Currency` (+ Amount (`self.Currency`))))
  (return _output_get))

(fn `SubtractCurrency`
  (params (Amount :type "Float (double-precision)"))
  (returns (NewCurrency :type "Float (double-precision)"))
  (locals (NewCurrencyLocal :type "Float (double-precision)"))
  (bind _output_get (set `self.Currency` (- (`self.Currency`) Amount)))
  (if (>= _output_get 0.0)
    (return (`self.Currency`))
    (else
      (bind _output_get_2 (set `self.Currency` 0.0))
      (return _output_get_2))))