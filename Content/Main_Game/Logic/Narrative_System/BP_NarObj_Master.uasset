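; Master Blueprint for narrative objects that appear at a random placed position and show a text pop-up when focused.
; The construction script applies mesh and material from the selected data table row, plus an outlined copy on the spawn-position preview mesh.
; On BeginPlay it picks a random text and teleports the mesh to a random child transform of ScenePositions.
; Focus toggles the custom depth stencil and pop-up, while Interact only returns false.
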(event `self.ReceiveBeginPlay`
  (bind (_structitem_mesh _structitem_material_inst _structitem_text) (break `/Game/Main_Game/Logic/Data/Notes/Struct_ItemNotes` (`self.StructItem`)))
  (`|ExecutionSequence`
    (:`then_0`
      (set `/Game/Main_Game/Logic/PopUp_Component.Text Pop Up` (`|GetArrayItem` _structitem_text (`KismetMathLibrary.RandomInteger` (`KismetArrayLibrary.Array_Length` _structitem_text))) (`self.PopUp_Component`)))
    (:`then_1`
      (for _array_element (`SceneComponent.GetChildrenComponents` (`self.ScenePositions`) false)
        (`KismetArrayLibrary.Array_AddUnique` (`self.ListLocationsToSpawn`) (`SceneComponent.K2_GetComponentToWorld` _array_element)))
      (`SceneComponent.K2_SetWorldTransform` (`self.StaticMesh`) (`KismetArrayLibrary.Array_Random` (`self.ListLocationsToSpawn`)) false true))))

(event `OnMouseEnter`
  (`/Game/Main_Game/Logic/PopUp_Component.ShowPopUp` (`self.PopUp_Component`)))

(event `OnMouseLeave`
  (`/Game/Main_Game/Logic/PopUp_Component.RemovePopUp` (`self.PopUp_Component`)))

(fn `Interact`
  (returns (Success :type Boolean))
  (return false))

(fn `Interact_ToggleFocus_T`
  (params (Focus :type Boolean))
  (returns (SubjectToAbility :type Boolean))
  (if Focus
    (`PrimitiveComponent.SetCustomDepthStencilValue` (`self.StaticMesh`) 0)
    (`self.OnMouseEnter`)
    (else
      (`PrimitiveComponent.SetCustomDepthStencilValue` (`self.StaticMesh`) 4)
      (`self.OnMouseLeave`)))
  (return (`self.Subject to Ability`)))

(fn `UserConstructionScript`
  (bind _outrownames (`DataTableFunctionLibrary.GetDataTableRowNames` (`self.Data`)))
  (set `self.OptionsNames` _outrownames)
  (bind _returnvalue (`|GetDataTableRow` (`self.Data`) (`self.SelectName`))
    (:`then`
      (set `self.StructItem` _returnvalue)
      (`|ExecutionSequence`
        (:`then_0`
          (bind (_mesh _material_inst) (break `/Game/Main_Game/Logic/Data/Notes/Struct_ItemNotes` _returnvalue))
          (`StaticMeshComponent.SetStaticMesh` (`self.StaticMesh`) _mesh)
          (for _array_element (`PrimitiveComponent.GetMaterialSlotNames` (`self.StaticMesh`))
            (`PrimitiveComponent.SetMaterialByName` (`self.StaticMesh`) _array_element _material_inst)))
        (:`then_1`
          (`StaticMeshComponent.SetStaticMesh` (`self.SpawnPositionMesh`) _mesh)
          (for _array_element_2 (`PrimitiveComponent.GetMaterialSlotNames` (`self.SpawnPositionMesh`))
            (`PrimitiveComponent.SetMaterialByName` (`self.SpawnPositionMesh`) _array_element_2 "/Game/Main_Game/Logic/Interaction_System/InteractionArea/M_DEV_Outline.M_DEV_Outline")))))))