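; Ability pickup that slows infection on the cube sections when the player touches it.
; When player character 0 overlaps its sphere, it finds every BP_CubeSection in the level and lengthens each InfectionTime by a quarter.
; It then destroys itself, making it a one-shot effect.
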(event `self.Sphere.OnComponentBeginOverlap`
  (params (OverlappedComponent :type "PrimitiveComponent Object Reference") (OtherActor :type "Actor Object Reference") (OtherComp :type "PrimitiveComponent Object Reference") (OtherBodyIndex :type Integer) (bFromSweep :type Boolean) (SweepResult :type "HitResult Structure (by ref)"))
  (if (== OtherActor (`GameplayStatics.GetPlayerCharacter` 0))
    (bind _outactors (`GameplayStatics.GetAllActorsOfClass` "/Game/Main_Game/Logic/A_Logic_Environment/BP_CubeSection.BP_CubeSection_C"))
    (for _array_element _outactors
      (set `/Game/Main_Game/Logic/A_Logic_Environment/BP_CubeSection.InfectionTime` (* (`/Game/Main_Game/Logic/A_Logic_Environment/BP_CubeSection.InfectionTime` _array_element) 1.25) _array_element))
    (`self.K2_DestroyActor`)))

(fn `UserConstructionScript`
  (`parent.UserConstructionScript`))