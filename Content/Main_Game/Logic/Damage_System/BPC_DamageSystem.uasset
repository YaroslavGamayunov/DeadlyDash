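; BPC_DamageSystem is a Blueprint component that tracks current health, maximum health and death state for damage handling.
; AddHealth changes current health within zero and the maximum, while AddMaxHealth raises the maximum, and both return the new value.
; TakeDamage reads the amount from a damage info input and, when it would be lethal, sets IsDead and calls OnDeath.
; Non-lethal damage leaves current health unchanged.
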(fn `Add Health`
  (params (Amount :type "Float (double-precision)"))
  (returns (NewHealth :type "Float (double-precision)"))
  (bind _output_get (set `self.Health_Current` (`KismetMathLibrary.FClamp` (+ Amount (`self.Health_Current`)) 0.0 (`self.Health_Max`))))
  (return _output_get))

(fn `AddMaxHealth`
  (params (Amount :type "Float (double-precision)"))
  (returns (NewMaxHealth :type "Float (double-precision)"))
  (bind _output_get (set `self.Health_Max` (+ Amount (`self.Health_Max`))))
  (return _output_get))

(fn `TakeDamage`
  (params (DamageInfo :type "/Game/Main_Game/Logic/Damage_System/S_DamageInfo Structure"))
  (if (<= (- (`self.Health_Current`) (`.Amount_2_F6570A254EE22CA5365476B5707F34F3` (break `/Game/Main_Game/Logic/Damage_System/S_DamageInfo` DamageInfo))) 0.0)
    (set `self.IsDead` true)
    (`self.OnDeath`)
    (return)))