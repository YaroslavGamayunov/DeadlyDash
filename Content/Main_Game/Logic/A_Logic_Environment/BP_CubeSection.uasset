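; BP_CubeSection is a floor or cube tile in a spreading infection hazard, started by a starter flag or Interact.
; A timeline scaled by InfectionTime blends the plane's material color while infected, and the player takes damage on entering its box.
; On finish, it damages a player still inside; otherwise it line-traces in four directions, calls Interact on hit actors to spread infection, then destroys itself.
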(event `self.ReceiveBeginPlay`
  (`|ExecutionSequence`
    (:`then_0`
      (if (`self.Infection Starter Section`)
        (`self.StartInfection`)))))

(event `StartInfection`
  (bind _returnvalue (`self.K2_GetActorLocation`))
  (set `self.Infected` true)
  (`TimelineComponent.SetPlayRate` (`self.Timeline`) (/ 1.0 (`self.InfectionTime`)))
  (bind (_direction _newtrack_0) (`Timeline|Timeline` :!via `PlayFromStart`)
    (:`Update`
      (`MeshComponent.SetScalarParameterValueOnMaterials` (`self.Plane`) "InnerColorLerp" (* _newtrack_0 1.0)))
    (:`Finished`
      (if (`self.CharacterIn`)
        (message `/Game/Main_Game/Logic/DamageSystem/BPI_Damagable.TakeDamage` (`GameplayStatics.GetPlayerCharacter` 0) (make `/Game/Main_Game/Logic/DamageSystem/S_DamageInfo` 5.0 "NewEnumerator1"))
        (else
          (`|ExecutionSequence`
            (:`then_0`
              (for _index (range 4)
                (bind _outhit (`KismetSystemLibrary.LineTraceSingleForObjects` :`Start` _returnvalue :`End` (+ _returnvalue (`KismetMathLibrary.GreaterGreater_VectorRotator` (`KismetMathLibrary.MakeVector` 250.0) (`KismetMathLibrary.MakeRotator` 0.0 0.0 (`KismetMathLibrary.Conv_IntToDouble` (* _index 90))))) :`ObjectTypes` (`|MakeArray` "ObjectTypeQuery1" "ObjectTypeQuery7" :!type "EObjectTypeQuery Enum") :`DrawDebugType` "ForDuration" :`DrawTime` 15.0))
                (message `/Game/Main_Game/Logic/Interfaces/Interactable_Interface.Interact` (`.HitActor` (`GameplayStatics.BreakHitResult` _outhit)))))
            (:`then_1`
              (`self.K2_DestroyActor`))))))))

(event `self.Box.OnComponentBeginOverlap`
  (params (OverlappedComponent :type "PrimitiveComponent Object Reference") (OtherActor :type "Actor Object Reference") (OtherComp :type "PrimitiveComponent Object Reference") (OtherBodyIndex :type Integer) (bFromSweep :type Boolean) (SweepResult :type "HitResult Structure (by ref)"))
  (bind _returnvalue (`GameplayStatics.GetPlayerCharacter` 0))
  (if (== OtherActor _returnvalue)
    (set `self.CharacterIn` true)
    (if (`self.Infected`)
      (message `/Game/Main_Game/Logic/DamageSystem/BPI_Damagable.TakeDamage` _returnvalue (make `/Game/Main_Game/Logic/DamageSystem/S_DamageInfo` 5.0 "NewEnumerator1")))))

(event `self.Box.OnComponentEndOverlap`
  (params (OverlappedComponent :type "PrimitiveComponent Object Reference") (OtherActor :type "Actor Object Reference") (OtherComp :type "PrimitiveComponent Object Reference") (OtherBodyIndex :type Integer))
  (if (== OtherActor (`GameplayStatics.GetPlayerCharacter` 0))
    (set `self.CharacterIn` false)))

(fn `Interact`
  (returns (Success :type Boolean))
  (`self.StartInfection`)
  (return true))

(fn `Interact_ToggleFocus_T`
  (params (Focus :type Boolean))
  (returns (SubjectToAbility :type Boolean))
  (return false))

(fn `UserConstructionScript`)