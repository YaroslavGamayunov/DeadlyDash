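; BP_Parent_Dash is, by its name, a base actor for dash objects, with a Cube that responds to interaction focus.
; BeginPlay caches the player character, and focus changes toggle the Cube's custom depth and swap its cursor-over material.
; HelperFutureGhost is an empty stub; its disconnected nodes would spawn a same-class ghost and add a screen-space line to the player's draw array, but never run.
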(event `self.ReceiveBeginPlay`
  (`|ExecutionSequence`
    (:`then_0`
      (bind _asbp_player_character (cast `/Game/Main_Game/Logic/A_Logic_Characters/Player/BP_PlayerCharacter` (`GameplayStatics.GetPlayerCharacter` 0)))
      (set `self.As BP Player Character` _asbp_player_character))))

(event `/Game/Main_Game/Logic/Interfaces/Interactable_Interface.Interact_ToggleFocus`
  (params (Focus :type Boolean))
  (`PrimitiveComponent.SetRenderCustomDepth` (`self.Cube`) Focus)
  (if Focus
    (`PrimitiveComponent.SetMaterial` (`self.Cube`) 0 (`self.BeginCursorOver_Mat`))
    (else
      (`PrimitiveComponent.SetMaterial` (`self.Cube`) 0 (`self.EndCursorOver_Mat`)))))

(fn `Helper | FutureGhost`
  (params (Class :type "Actor Class Reference")))

(fn `UserConstructionScript`)