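; Surface portal to the CodeZone that starts a level as soon as something overlaps its box.
; The overlap feeds GetSeed and IncreaseLevel, neither defined here, into StartLevel at the zero position.
; A separate function increments and saves the CodeZone cycle count while preserving other zones' story progress, but nothing here calls it.
; Interaction and focus overrides return false, and the respawn timeline function is empty.
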(event `self.Box.OnComponentBeginOverlap`
  (params (OverlappedComponent :type "PrimitiveComponent Object Reference") (OtherActor :type "Actor Object Reference") (OtherComp :type "PrimitiveComponent Object Reference") (OtherBodyIndex :type Integer) (bFromSweep :type Boolean) (SweepResult :type "HitResult Structure (by ref)"))
  (bind _returnvalue (`CurrentSessionData.GetSeed`))
  (bind _returnvalue_2 (`CurrentSessionData.IncreaseLevel`))
  (`GameLoader.StartLevel` _returnvalue _returnvalue_2))

(fn `Interact`
  (params (`Actor Causer` :type "Actor Object Reference"))
  (returns (Success :type Boolean))
  (return false))

(fn `Interact_ToggleFocus_T`
  (params (Focus :type Boolean))
  (returns (SubjectToAbility :type Boolean))
  (return false))

(fn `Play_WorldRespawn_TL`
  (params (Forward :type Boolean)))

(fn `SaveAndProgressCycleNumber`
  (bind _returnvalue (`GameplayStatics.GetGameInstance`))
  (bind _savegamedata (message `/Game/Main_Game/Logic/SaveGame/BPI_SaveGame.GetGameData` _returnvalue))
  (bind (_zones_save_cz_cycle_current _zones_save_orgzonestoryprogress _zones_save_techzonestoryprogress _zones_save_sandzonestoryprogress) (break `/Game/Main_Game/Logic/SaveGame/S_ZonesSave` (`/Game/Main_Game/Logic/SaveGame/BP_SaveGame.Zones_Save` _savegamedata)))
  (bind _result (`/Engine/EditorBlueprintResources/StandardMacros.IncrementInt` _zones_save_cz_cycle_current)
    (:`  `
      (message `/Game/Main_Game/Logic/SaveGame/BPI_SaveGame.SaveZonesData` _returnvalue (make `/Game/Main_Game/Logic/SaveGame/S_ZonesSave` _result _zones_save_orgzonestoryprogress _zones_save_techzonestoryprogress _zones_save_sandzonestoryprogress) false))))

(fn `UserConstructionScript`
  (`parent.UserConstructionScript`)
  (`self.SetActorHiddenInGame` false))