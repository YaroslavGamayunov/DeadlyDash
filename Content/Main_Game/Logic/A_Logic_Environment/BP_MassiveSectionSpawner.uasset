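; BP_MassiveSectionSpawner is an actor that fills an area with a flat grid of BP_CubeSection actors.
; On BeginPlay it loops over HorizontalAmount times VerticalAmount, spawning sections at fixed spacing from its own location.
; X derives from index divided by VerticalAmount and Y from index modulo HorizontalAmount, so the grid is only regular when both match.
; A construction-script version using static mesh components is left disconnected.
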(event `self.ReceiveBeginPlay`
  (bind (_returnvalue_x _returnvalue_y _returnvalue_z) (`KismetMathLibrary.BreakVector` (`self.K2_GetActorLocation`)))
  (bind _output_get (set `self.OverallCounter` (- (* (`self.Horizontal Amount`) (`self.Vertical Amount`)) 1)))
  (for _index (range (+ _output_get 1))
    (`|SpawnActorFromClass` "/Game/Main_Game/Logic/A_Logic_Environment/BP_CubeSection.BP_CubeSection_C" (`KismetMathLibrary.MakeTransform` (`KismetMathLibrary.MakeVector` (+ (`KismetMathLibrary.Conv_IntToDouble` (* (/ _index (`self.Vertical Amount`)) 250)) _returnvalue_x) (+ (`KismetMathLibrary.Conv_IntToDouble` (* (mod _index (`self.Horizontal Amount`)) 250)) _returnvalue_y) _returnvalue_z)) "AlwaysSpawn" "MultiplyWithRoot" null null)))

(fn `UserConstructionScript`)