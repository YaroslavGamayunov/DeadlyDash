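; Portal actor that saves the player and sends them to the Instructor, Code or Alive Zone on first overlap.
; An optional currency timer widget stops on entry to award currency, and can be frozen temporarily.
; Material-parameter timelines play a world-appear effect after scene load and reverse before travel, varying by current level type.
; Instructor travel advances the saved cycle, Code picks a random level for that cycle, and Alive pauses into a traveler widget.
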(event `self.ReceiveBeginPlay`
  (bind _az_levels (`/Game/Main_Game/Logic/Data/Levels/PDA_LevelsTraveler.AZ_Levels` (`self.PDA_Levels`)))
  (`|ExecutionSequence`
    (:`then_0`
      (if (`self.SpawnTimer`)
        (bind _returnvalue (`|CreateWidget` "/Game/Main_Game/UI/Blueprints/WB_CurrencyTimer.WB_CurrencyTimer_C" null (`self.Max Time`)))
        (bind _output_get (set `self.WB_CurrencyTimer` _returnvalue))
        (`UserWidget.AddToViewport` _output_get 0)))
    (:`then_1`
      (bind _returnvalue_2 (`GameplayStatics.GetCurrentLevelName` true))
      (bind _keys (`BlueprintMapLibrary.Map_Keys` _az_levels))
      (for _array_element _keys
        (if (`KismetArrayLibrary.Array_Contains` (`.L_Names_Array_14_579AC3DD4639C347023CE28865F3D9C5` (break `/Game/Main_Game/Logic/Data/Levels/S_LevelsTraveler` (`BlueprintMapLibrary.Map_Find` _az_levels _array_element))) (`KismetStringLibrary.Conv_StringToName` _returnvalue_2))
          (set `self.CurrentLevelType_AZ` true)
          (break))))
    (:`then_2`
      (bind _returnvalue_3 (`GameplayStatics.GetActorOfClass` "/Game/Main_Game/Logic/Systems/Narrative_System/SceneManager.SceneManager_C"))
      (`/Engine/EditorBlueprintResources/StandardMacros.IsValid` _returnvalue_3
        (:`Is Valid`
          (add `/Game/Main_Game/Logic/Systems/Narrative_System/SceneManager.OnStreamLevelLoad` _returnvalue_3 (delegate `Play_WR_TL`))
          (`/Game/Main_Game/Logic/Systems/Narrative_System/SceneManager.LoadScene` _returnvalue_3))
        (:`Is Not Valid`
          (`KismetSystemLibrary.Delay` 1.5 :!label _label)
          (`self.Play_WorldRespawn_TL` true))))))

(event `Play_WR_TL`
  (goto _label))

(event `FreezeTime`
  (bind _wb_currencytimer (`self.WB_CurrencyTimer`))
  (set `/Game/Main_Game/UI/Blueprints/WB_CurrencyTimer.TimerActive` false _wb_currencytimer)
  (`KismetSystemLibrary.Delay` 15.0)
  (set `/Game/Main_Game/UI/Blueprints/WB_CurrencyTimer.TimerActive` true _wb_currencytimer))

(event `To IZ level`
  (`/Game/Main_Game/Logic/MacroLibraries/BML_Object.AsyncOpenLevel_byStruct` (`/Game/Main_Game/Logic/Data/Levels/PDA_LevelsTraveler.IZ_Level` (`self.PDA_Levels`))))

(event `self.Box.OnComponentBeginOverlap`
  (params (OverlappedComponent :type "PrimitiveComponent Object Reference") (OtherActor :type "Actor Object Reference") (OtherComp :type "PrimitiveComponent Object Reference") (OtherBodyIndex :type Integer) (bFromSweep :type Boolean) (SweepResult :type "HitResult Structure (by ref)"))
  (bind _returnvalue (`GameplayStatics.GetGameInstance`))
  (bind _wb_currencytimer (`self.WB_CurrencyTimer`))
  (if (== OtherActor (`GameplayStatics.GetPlayerCharacter` 0))
    (`/Engine/EditorBlueprintResources/StandardMacros.DoOnce` false
      (:`Completed`
        (if (`self.SpawnTimer`)
          (set `/Game/Main_Game/UI/Blueprints/WB_CurrencyTimer.TimerActive` false _wb_currencytimer)
          (message `/Game/Main_Game/Logic/Systems/Currency_System/BPI_Currencyable.AddCurrency` (`GameplayStatics.GetPlayerCharacter` 0) (`KismetMathLibrary.Conv_IntToDouble` (`/Game/Main_Game/UI/Blueprints/WB_CurrencyTimer.MaxTime_Int` _wb_currencytimer))))
        (bind _asbp_player_character_parent (cast `/Game/Main_Game/Logic/A_Logic_Characters/Player/BP_PlayerCharacter_Parent` (`GameplayStatics.GetPlayerCharacter` 0)))
        (`/Game/Main_Game/Logic/A_Logic_Characters/Player/BP_PlayerCharacter_Parent.SavePlayerData` _asbp_player_character_parent false)
        (switch `/Game/Main_Game/Logic/Data/Levels/E_ZoneTypes` (`self.ZoneTypeToTravel`)
          (:`NewEnumerator0`
            ;[1 1 1] Save and progress Cycle number
            (bind _savegamedata (message `/Game/Main_Game/Logic/SaveGame/BPI_SaveGame.GetGameData` _returnvalue))
            (bind (_zones_save_cz_cycle_current _zones_save_orgzonestoryprogress _zones_save_techzonestoryprogress _zones_save_sandzonestoryprogress) (break `/Game/Main_Game/Logic/SaveGame/S_ZonesSave` (`/Game/Main_Game/Logic/SaveGame/BP_SaveGame.Zones_Save` _savegamedata)))
            (bind _result (`/Engine/EditorBlueprintResources/StandardMacros.IncrementInt` _zones_save_cz_cycle_current)
              (:`  `
                (message `/Game/Main_Game/Logic/SaveGame/BPI_SaveGame.SaveZonesData` _returnvalue (make `/Game/Main_Game/Logic/SaveGame/S_ZonesSave` _result _zones_save_orgzonestoryprogress _zones_save_techzonestoryprogress _zones_save_sandzonestoryprogress) false)
                (add `self.On PP_TL End` (delegate `To IZ level`))
                (`self.Play_WorldRespawn_TL` false))))
          (:`NewEnumerator1`
            (bind _savegamedata_2 (message `/Game/Main_Game/Logic/SaveGame/BPI_SaveGame.GetGameData` (`GameplayStatics.GetGameInstance`)))
            (bind _zones_save_cz_cycle_current_2 (break `/Game/Main_Game/Logic/SaveGame/S_ZonesSave` (`/Game/Main_Game/Logic/SaveGame/BP_SaveGame.Zones_Save` _savegamedata_2)))
            (bind _value (`/Game/Main_Game/Logic/Data/Levels/PDA_LevelsTraveler.Get CZ level` (`self.PDA_Levels`) _zones_save_cz_cycle_current_2))
            (set `self.Current Level Index` (`.OutIndex` (`KismetArrayLibrary.Array_Random` (`.L_SObjects_Array_13_15552F8A4C7B20844FC5E3A1690A2204` (break `/Game/Main_Game/Logic/Data/Levels/S_LevelsTraveler` _value)))))
            (add `self.On PP_TL End` (delegate `To CZ level`))
            (`self.Play_WorldRespawn_TL` false))
          (:`NewEnumerator2`
            (add `self.On PP_TL End` (delegate `To AZ level`))
            (`self.Play_WorldRespawn_TL` false)))))))

(event `To CZ level`
  (`/Game/Main_Game/Logic/MacroLibraries/BML_Object.AsyncOpenLevel_byStruct` (stale `self.Box.OnComponentBeginOverlap` _value) (`self.Current Level Index`)))

(event `To AZ level`
  (`GameplayStatics.SetGamePaused` true)
  (bind _returnvalue (`|CreateWidget` "/Game/Main_Game/UI/Blueprints/WB_AZ_Traveler.WB_AZ_Traveler_C"))
  (`UserWidget.AddToViewport` _returnvalue 0))

(fn `Interact`
  (params (`Actor Causer` :type "Actor Object Reference"))
  (returns (Success :type Boolean))
  (return false))

(fn `Interact_ToggleFocus_T`
  (params (Focus :type Boolean))
  (returns (SubjectToAbility :type Boolean))
  (return false))

(fn `Play_WorldRespawn_TL`
  (params (Forward :type Boolean))
  (if Forward
    (if (`self.CurrentLevelType_AZ`)
      (`TimelineComponent.PlayFromStart` (`self.TL_respawn_AZ`))
      (else
        (`TimelineComponent.PlayFromStart` (`self.TL_respawn_CZ`))))
    (elif (`self.CurrentLevelType_AZ`)
      (`TimelineComponent.ReverseFromEnd` (`self.TL_respawn_AZ`))
      (else
        (`TimelineComponent.ReverseFromEnd` (`self.TL_respawn_CZ`)))))
  (return))

(fn `UserConstructionScript`
  (`parent.UserConstructionScript`)
  (`self.SetActorHiddenInGame` (`self.HiddenInGame`)))