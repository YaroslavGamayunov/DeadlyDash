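; BP_Parent_Dash is a parent Blueprint, filed under arrow movement, for an interactable Plane that highlights on focus.
; Interact calls an InteractEvent, whose handler in this Blueprint is empty.
; The focus toggle switches the Plane's custom depth rendering and swaps between cursor-over and cursor-end materials.
; Custom depth stencil writes are present but disconnected, so they never run.
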(event `Interact_Event`)

(fn `Interact`
  (returns (Success :type Boolean))
  (`self.Interact_Event`)
  (return false))

(fn `Interact_ToggleFocus_T`
  (params (Focus :type Boolean))
  (returns (SubjectToAbility :type Boolean))
  (`PrimitiveComponent.SetRenderCustomDepth` (`self.Plane`) Focus)
  (if Focus
    (`PrimitiveComponent.SetMaterial` (`self.Plane`) 0 (`self.BeginCursorOver_Mat`))
    (else
      (`PrimitiveComponent.SetMaterial` (`self.Plane`) 0 (`self.EndCursorOver_Mat`))))
  (return false))

(fn `UserConstructionScript`)