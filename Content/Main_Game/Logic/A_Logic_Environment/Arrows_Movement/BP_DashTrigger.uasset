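; BP_DashTrigger is an interactable trigger that dashes the top-down player character along the trigger's rotation.
; It caches the player on BeginPlay, and only InteractEvent performs the dash.
; Both interaction and LeftTheScreen then tell the player's DashSpawnerComponent to spawn a dash using the trigger's yaw, play an explosion effect and destroy the actor.
; A Clicked flag ensures only the first of these events takes effect.
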(event `self.ReceiveBeginPlay`
  (`parent.ReceiveBeginPlay`)
  (bind _asbp_player_character_top_down (cast `/Game/Main_Game/Logic/A_Logic_Characters/Player/BP_PlayerCharacterTopDown` (`GameplayStatics.GetPlayerCharacter` 0)))
  (set `self.As BP Player Character Top Down` _asbp_player_character_top_down))

(event `LeftTheScreen`
  (if (not (`self.Clicked`))
    (set `self.Clicked` true)
    (`/Game/Main_Game/Logic/A_Logic_Characters/Player/DashSpawner_Component.SpawnDash | afterDisappear` (`/Game/Main_Game/Logic/A_Logic_Characters/Player/BP_PlayerCharacterTopDown.DashSpawner_Component` (`self.As BP Player Character Top Down`)) (.yaw (`self.K2_GetActorRotation`)) :!label _label)
    (`GameplayStatics.SpawnEmitterAtLocation` "/Game/Starter/StarterContent/Particles/P_Explosion.P_Explosion" (`self.K2_GetActorLocation`))
    (`self.K2_DestroyActor`)))

(event `self.Interact_Event`
  (`parent.Interact_Event`)
  (if (not (`self.Clicked`))
    (set `self.Clicked` true)
    (`/Game/Main_Game/Logic/A_Logic_Characters/Player/BP_PlayerCharacterTopDown.Dash` (`self.As BP Player Character Top Down`) (`self.K2_GetActorRotation`))
    (goto _label)))

(fn `UserConstructionScript`
  (`parent.UserConstructionScript`))