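; BP_Arrow_P is a clickable arrow, apparently a parent for environment movement arrows, that responds to interact and focus calls.
; Interacting activates its Niagara effect, fires the OnArrowClick dispatcher and calls an interact event, which is empty here.
; Focus changes swap the plane's material between cursor-over and cursor-out versions and toggle its custom depth stencil value.
; The node that would toggle custom depth rendering is disconnected.
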(event `Interact_Event`)

(fn `Interact`
  (params (`Actor Causer` :type "Actor Object Reference"))
  (returns (Success :type Boolean))
  (`ActorComponent.Activate` (`self.Niagara`) false)
  (`self.OnArrowClick`)
  (`self.Interact_Event`)
  (return false))

(fn `Interact_ToggleFocus_T`
  (params (Focus :type Boolean))
  (returns (SubjectToAbility :type Boolean))
  (bind _plane (`self.Plane`))
  (if Focus
    (`PrimitiveComponent.SetCustomDepthStencilValue` _plane 1)
    (`PrimitiveComponent.SetMaterial` (`self.Plane`) 0 (`self.BeginCursorOver_Mat`))
    (else
      (`PrimitiveComponent.SetCustomDepthStencilValue` _plane 0)
      (`PrimitiveComponent.SetMaterial` (`self.Plane`) 0 (`self.EndCursorOver_Mat`))))
  (return false))

(fn `UserConstructionScript`)