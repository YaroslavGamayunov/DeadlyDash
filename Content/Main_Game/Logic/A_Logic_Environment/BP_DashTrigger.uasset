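; BP_DashTrigger is a one-shot dash trigger actor that dashes the player along its own rotation when interacted with.
; Interact calls Dash on the player, while LeftTheScreen skips the dash; a Clicked flag lets only the first event act.
; Both paths then pass the trigger's yaw to the player's DashSpawnerComponent via SpawnDashAfterDisappear, spawn an explosion emitter and destroy the actor.
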(event `LeftTheScreen`
  (if (not (`self.Clicked`))
    (set `self.Clicked` true)
    (`/Game/Main_Game/Logic/A_Logic_Characters/Player/DashSpawner_Component.SpawnDash | afterDisappear` (`/Game/Main_Game/Logic/A_Logic_Characters/Player/BP_PlayerCharacter.DashSpawner_Component` (`self.As BP Player Character`)) (.yaw (`self.K2_GetActorRotation`)) :!label _label)
    (`GameplayStatics.SpawnEmitterAtLocation` "/Game/Starter/StarterContent/Particles/P_Explosion.P_Explosion" (`self.K2_GetActorLocation`))
    (`self.K2_DestroyActor`)))

(event `/Game/Main_Game/Logic/Interfaces/Interactable_Interface.Interact`
  (if (not (`self.Clicked`))
    (set `self.Clicked` true)
    (`/Game/Main_Game/Logic/A_Logic_Characters/Player/BP_PlayerCharacter.Dash` (`self.As BP Player Character`) (`self.K2_GetActorRotation`))
    (goto _label)))

(fn `UserConstructionScript`
  (`parent.UserConstructionScript`))