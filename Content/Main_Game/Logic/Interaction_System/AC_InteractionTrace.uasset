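; Interaction component that traces every tick to find the interaction area under the first-person camera's view or the top-down mouse cursor.
; When the traced actor changes, it moves focus between box or custom-shape interaction areas and fires mouse enter and leave calls.
; TryToInteract sends InteractMessage to the focused area's parent actor and returns that actor on success.
; A narrative-object branch is left unconnected.
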(event `self.ReceiveBeginPlay`
  (if (`self.FirstPerson?`)
    (bind _asbp_player_character_first_person (cast `/Game/Main_Game/Logic/A_Logic_Characters/Player/BP_PlayerCharacterFirstPerson` (`GameplayStatics.GetPlayerCharacter` 0)))
    (set `self.First Person Camera` (`/Game/Main_Game/Logic/A_Logic_Characters/Player/BP_PlayerCharacterFirstPerson.FirstPersonCamera` _asbp_player_character_first_person))))

(event `self.ReceiveTick`
  (params (DeltaSeconds :type "Float (single-precision)"))
  (if (`self.FirstPerson?`)
    (bind (_outhit _returnvalue) (`self.TraceSetting_FirstPerson`))
    (`self.TraceLogic` _returnvalue _outhit)
    (else
      (bind (_outhit_2 _returnvalue_2) (`self.TraceSetting_TopDown`))
      (`self.TraceLogic` _returnvalue_2 _outhit_2))))

(fn `InteractionArea`
  (params (Trace :type Boolean))
  (if Trace
    (if (`self.IsTracingTheActor`)
      (bind _focused_interaction_area (`self.Focused_Interaction Area`)
        (:`then`
          (bind _subjecttoability (`/Game/Main_Game/Logic/Interaction_System/InteractionArea/BP_InteractionArea_Master.ToggleFocus` _focused_interaction_area false))
          (if _subjecttoability
            (`self.OnMouseLeave`)))
        (:`else`
          _)))
    (bind _asbp_interaction_area_master (cast `/Game/Main_Game/Logic/Interaction_System/InteractionArea/BP_InteractionArea_Master` (`self.FocusedActor`)))
    (bind _output_get (set `self.Focused_Interaction Area` _asbp_interaction_area_master))
    (bind _subjecttoability_2 (`/Game/Main_Game/Logic/Interaction_System/InteractionArea/BP_InteractionArea_Master.ToggleFocus` _output_get true))
    (if _subjecttoability_2
      (`self.OnMouseEnter`))
    (set `self.IsTracingTheActor` true)
    (elif (`self.IsTracingTheActor`)
      (bind _focused_interaction_area_2 (`self.Focused_Interaction Area`)
        (:`then`
          (bind _subjecttoability_3 (`/Game/Main_Game/Logic/Interaction_System/InteractionArea/BP_InteractionArea_Master.ToggleFocus` _focused_interaction_area_2 false))
          (if _subjecttoability_3
            (`self.OnMouseLeave`)))
        (:`else`
          _))
      (set `self.IsTracingTheActor` false)
      (set `self.FocusedActor` null)
      (set `self.Focused_Interaction Area` null)
      (set `self.Focused Nar Obj` null)
      (set `self.NarrativeObj` false))))

(fn `TraceLogic`
  (params (Condition :type Boolean) (Hit :type "HitResult Structure (by ref)"))
  (bind (_bblockinghit _binitialoverlap _time _distance _location _impactpoint _normal _impactnormal _physmat _hitactor) (`GameplayStatics.BreakHitResult` Hit))
  (bind _focusedactor (`self.FocusedActor`))
  (bind _returnvalue (`GameplayStatics.GetObjectClass` _hitactor))
  (if Condition
    (if (!= _focusedactor _hitactor)
      (`self.FocusedActor`
        (:`then`
          (if (!= (`Actor.GetParentActor` _focusedactor) (`Actor.GetParentActor` _hitactor))
            (set `self.FocusedActor` _hitactor :!label _label)
            (`self.InteractionArea` (or (== _returnvalue "/Game/Main_Game/Logic/Interaction_System/InteractionArea/BP_InteractionArea_CustomShape.BP_InteractionArea_CustomShape_C") (== _returnvalue "/Game/Main_Game/Logic/Interaction_System/InteractionArea/BP_InteractionArea_BoxShape.BP_InteractionArea_BoxShape_C")))))
        (:`else`
          (goto _label))))
    (else
      (`self.InteractionArea` false))))

(fn `TraceSetting_FirstPerson`
  (returns (OutHit :type "HitResult Structure") (ReturnValue :type Boolean))
  (bind _first_person_camera (`self.First Person Camera`))
  (bind _returnvalue (`SceneComponent.K2_GetComponentLocation` _first_person_camera))
  (bind (_outhit _returnvalue_2) (`KismetSystemLibrary.LineTraceSingle` :`Start` _returnvalue :`End` (+ _returnvalue (* (`SceneComponent.GetForwardVector` _first_person_camera) 10000)) :`TraceChannel` "TraceTypeQuery1" :`DrawDebugType` "ForOneFrame"))
  (return _outhit _returnvalue_2))

(fn `TraceSetting_TopDown`
  (returns (OutHit :type "HitResult Structure") (ReturnValue :type Boolean))
  (bind (_outhit _returnvalue) (`KismetSystemLibrary.LineTraceSingle` (`PlayerController.DeprojectMousePositionToWorld` (`GameplayStatics.GetPlayerController` 0)) (`/Game/Main_Game/Logic/CoreUtils/BFL_NewNodes.Get Mouse projection on Z plane` (`self.Z Plane | Trace`)) "TraceTypeQuery1"))
  (return _outhit _returnvalue))

(fn `TryToInteract`
  (returns (Success :type Boolean) (ActorInteracted :type "Actor Object Reference"))
  (bind _focused_interaction_area (`self.Focused_Interaction Area`))
  (bind _returnvalue (`Actor.GetParentActor` _focused_interaction_area))
  (if (`self.IsTracingTheActor`)
    (`/Engine/EditorBlueprintResources/StandardMacros.IsValid` _focused_interaction_area
      (:`Is Valid`
        (bind _success (message `/Game/Main_Game/Logic/Interfaces/Interactable_Interface.Interact` _returnvalue))
        (if _success
          (bind _output_get (set `self.InteractedActor` _returnvalue))
          (return _success _output_get)
          (else
            _)))
      (:`Is Not Valid`
        _))
    (return false null)))