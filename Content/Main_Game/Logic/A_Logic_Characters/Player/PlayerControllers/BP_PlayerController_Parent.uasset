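; Parent player controller that handles mouse clicks in the world and gives audiovisual feedback for each one.
; On BeginPlay it fetches and stores a reference to the base HUD.
; IA_Click line-traces from the projected mouse position to a plane just below Z zero, choosing the sound by whether it hits an interaction area.
; ClickEffect plays that sound and spawns an explosion emitter at the impact point, or at the trace end on a miss.
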(event `self.ReceiveBeginPlay`
  (bind _asbp_hud_base (`/Game/Main_Game/Logic/BML_PlayerController.Get BP HUD Base` 10.0)
    (:`Success`
      (set `self.As BP HUD Base` _asbp_hud_base))))

(event `EnhancedInput|/Game/Main_Game/Input/Actions/IA_Click`
  (params (ActionValue :type Boolean) (ElapsedSeconds :type "Float (double-precision)") (TriggeredSeconds :type "Float (double-precision)") (InputAction :type "InputAction Object Reference" :default "/Game/Main_Game/Input/Actions/IA_Click.IA_Click"))
  (:`Started`
    (bind _outhit (`KismetSystemLibrary.LineTraceSingle` (`/Game/Main_Game/Logic/CoreUtils/BFL_NewNodes.Get Mouse projection in Space`) (`/Game/Main_Game/Logic/CoreUtils/BFL_NewNodes.Get Mouse projection on Z plane` -10.0) "TraceTypeQuery1"))
    (cast `/Game/Main_Game/Logic/InteractionSystem/InteractionArea/BP_InteractionArea_Master` (`.HitActor` (`GameplayStatics.BreakHitResult` _outhit))
      (:`then`
        (`self.ClickEffect` _outhit "/Engine/VREditor/Sounds/UI/Scaling_Down.Scaling_Down" "/Game/Starter/StarterContent/Particles/P_Explosion.P_Explosion"))
      (:`CastFailed`
        (`self.ClickEffect` _outhit "/Engine/VREditor/Sounds/UI/Laser_Push.Laser_Push" "/Game/Starter/StarterContent/Particles/P_Explosion.P_Explosion")))))

(event `self.ReceiveTick`
  (params (DeltaSeconds :type "Float (single-precision)")))

(fn `UserConstructionScript`)