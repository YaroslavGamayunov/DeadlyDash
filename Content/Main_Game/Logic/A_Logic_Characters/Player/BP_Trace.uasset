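; BP_Trace is an actor that acts as a damaging trail left by the player's dash.
; It anchors one end at the player's start location, and a timeline scaled to DashDuration line-traces from the moving player to it, damaging Pawns hit.
; When the timeline finishes or is stopped early, the line freezes and a looping timer keeps tracing it for a residual duration before the actor destroys itself.
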(event `self.ReceiveBeginPlay`
  (bind _as_bp_player_character (`self.As BP Player Character`))
  (bind _asbp_player_character (cast `/Game/Main_Game/Logic/A_Logic_Characters/Player/BP_PlayerCharacter` (`GameplayStatics.GetPlayerCharacter` 0)))
  (set `self.As BP Player Character` _asbp_player_character)
  (set `self.EndTrace` (`self.K2_GetActorLocation` _as_bp_player_character) :!label _label)
  (`TimelineComponent.SetPlayRate` (`self.Timeline`) (/ 1.0 (`/Game/Main_Game/Logic/A_Logic_Characters/Player/BP_PlayerCharacter.Dash_Duration` _as_bp_player_character)))
  (`Timeline|Timeline` :!via `PlayFromStart`
    (:`Update`
      (`self.Trail_MultiLineTrace` (`self.K2_GetActorLocation` (`self.As BP Player Character`))))
    (:`Finished`
      (set `self.Start Trace` (`self.K2_GetActorLocation` (`self.As BP Player Character`)) :!label _label_2)
      (bind _returnvalue (`KismetSystemLibrary.K2_SetTimerDelegate` (delegate `ResidualTrail`) 0.01 true))
      (set `self.Trail_Live_Timer` _returnvalue)
      (`KismetSystemLibrary.Delay` (+ 5.0 (* (`/Game/Main_Game/Logic/A_Logic_Characters/Player/BP_PlayerCharacter.Dash_Duration` (`self.As BP Player Character`)) (- (`self.TL_PlaybackPosition`) 1.0))))
      (`KismetSystemLibrary.K2_ClearAndInvalidateTimerHandle` (`self.Trail_Live_Timer`))
      (`self.K2_DestroyActor`))))

(event `Trail`
  (goto _label))

(event `stop`
  (bind _timeline (`self.Timeline`))
  ;[0.1406 0.1406 0.1406] Преждевременная остановка следа
  (if (`TimelineComponent.IsPlaying` _timeline)
    (set `self.TL_PlaybackPosition` (`TimelineComponent.GetPlaybackPosition` _timeline))
    (`TimelineComponent.Stop` _timeline)
    (`self.Timer Residual Trail`)))

(event `Timer Residual Trail`
  (goto _label_2))

(event `ResidualTrail`
  (`self.Trail_MultiLineTrace` (`self.Start Trace`)))

(fn `Trail_MultiLineTrace`
  (params (`Start Trace` :type "Vector Structure"))
  (bind (_outhits _returnvalue) (`KismetSystemLibrary.LineTraceMultiForObjects` `Start Trace` (`self.EndTrace`) (`|MakeArray` "ObjectTypeQuery3" :!type "EObjectTypeQuery Enum") false (`|MakeArray` (`self.As BP Player Character`) :!type "Actor Object Reference") "ForOneFrame" true (struct :`R` 1.0 :`A` 1.0) (struct :`G` 1.0 :`A` 1.0) 0.0))
  (if _returnvalue
    (for _array_element _outhits
      (bind (_bblockinghit _binitialoverlap _time _distance _location _impactpoint _normal _impactnormal _physmat _hitactor) (`GameplayStatics.BreakHitResult` _array_element))
      (`GameplayStatics.ApplyDamage` _hitactor 1.0 null (`self.As BP Player Character`))
      (`KismetSystemLibrary.PrintString` (`KismetSystemLibrary.GetDisplayName` _hitactor)))))

(fn `UserConstructionScript`)