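; Parent player character Blueprint that wraps damage, currency, ability and interaction components behind pass-through functions for health, damage and currency.
; On BeginPlay it loads health and currency from the game instance, with a matching event to write them back, and adds a debug ability.
; Click input spawns a Test actor and attempts trace-based interaction.
; The damage component's death delegate is bound in the construction script; the Death event is empty.
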(event `self.ReceiveBeginPlay`
  (`|ExecutionSequence`
    (:`then_0`
      (bind _asmain_game_instanse (cast `/Game/Main_Game/MainGameInstanse` (`GameplayStatics.GetGameInstance`)))
      (set `self.As Main Game Instanse` _asmain_game_instanse)
      (`self.VariablesFromGI`))
    (:`then_1`
      ;[1 1 1] debug - delete
      (`/Game/Main_Game/Logic/AbilitySystem/AbilityManager/BPC_AbilityManager.AddAbility` (`self.BPC_AbilityManager`) (`self.Class`)))))

(event `EnhancedInput|/Game/Main_Game/Input/Actions/IA_Click`
  (params (ActionValue :type Boolean) (ElapsedSeconds :type "Float (double-precision)") (TriggeredSeconds :type "Float (double-precision)") (InputAction :type "InputAction Object Reference" :default "/Game/Main_Game/Input/Actions/IA_Click.IA_Click"))
  (:`Started`
    (`|SpawnActorFromClass` "/Game/Main_Game/Logic/A_Logic_Characters/Player/test.test_C" (`KismetMathLibrary.MakeTransform` (`self.K2_GetActorLocation`) (`SceneComponent.K2_GetComponentRotation` (`self.Mesh`))) "Undefined" "MultiplyWithRoot" null null)
    (bind _success (`/Game/Main_Game/Logic/InteractionSystem/AC_InteractionTrace.TryToInteract` (`self.AC_InteractionTrace`)))
    (if _success
      (`self.OnClick`))))

(event `Death`)

(event `VariablesFromGI`
  (bind _bpc_damagesystem (`self.BPC_DamageSystem`))
  (bind _as_main_game_instanse (`self.As Main Game Instanse`))
  (set `/Game/Main_Game/Logic/DamageSystem/BPC_DamageSystem.Health_Max` (`/Game/Main_Game/MainGameInstanse.HitPoints_Max` _as_main_game_instanse) _bpc_damagesystem)
  (set `/Game/Main_Game/Logic/DamageSystem/BPC_DamageSystem.Health_Current` (`/Game/Main_Game/MainGameInstanse.HitPoints_Current` _as_main_game_instanse) _bpc_damagesystem)
  (set `/Game/Main_Game/Logic/CurrencySystem/BPC_CurrencySystem.Currency` (`/Game/Main_Game/MainGameInstanse.Currency` _as_main_game_instanse) (`self.BPC_CurrencySystem`)))

(event `VariablesToGI`
  (bind _as_main_game_instanse (`self.As Main Game Instanse`))
  (bind _bpc_damagesystem (`self.BPC_DamageSystem`))
  (set `/Game/Main_Game/MainGameInstanse.HitPoints_Max` (`/Game/Main_Game/Logic/DamageSystem/BPC_DamageSystem.Health_Max` _bpc_damagesystem) _as_main_game_instanse)
  (set `/Game/Main_Game/MainGameInstanse.HitPoints_Current` (`/Game/Main_Game/Logic/DamageSystem/BPC_DamageSystem.Health_Current` _bpc_damagesystem) _as_main_game_instanse)
  (set `/Game/Main_Game/MainGameInstanse.Currency` (`/Game/Main_Game/Logic/CurrencySystem/BPC_CurrencySystem.Currency` (`self.BPC_CurrencySystem`)) _as_main_game_instanse))

(fn `AddCurrency`
  (params (Amount :type "Float (double-precision)"))
  (returns (NewCurrency :type "Float (double-precision)"))
  (bind _newcurrency (`/Game/Main_Game/Logic/CurrencySystem/BPC_CurrencySystem.AddCurrency` (`self.BPC_CurrencySystem`) Amount))
  (return _newcurrency))

(fn `AddHealth`
  (params (Amount :type "Float (double-precision)"))
  (returns (NewHealth :type "Float (double-precision)"))
  (bind _newhealth (`/Game/Main_Game/Logic/DamageSystem/BPC_DamageSystem.Add Health` (`self.BPC_DamageSystem`) Amount))
  (return _newhealth))

(fn `AddMaxHealth`
  (params (Amount :type "Float (double-precision)"))
  (returns (NewMaxHealth :type "Float (double-precision)"))
  (bind _newmaxhealth (`/Game/Main_Game/Logic/DamageSystem/BPC_DamageSystem.AddMaxHealth` (`self.BPC_DamageSystem`) Amount))
  (return _newmaxhealth))

(fn `Get Current Health`
  (returns (CurrentHealth :type "Float (double-precision)"))
  (return (`/Game/Main_Game/Logic/DamageSystem/BPC_DamageSystem.Health_Current` (`self.BPC_DamageSystem`))))

(fn `GetCurrentCurrency`
  (returns (CurrentCurrency :type "Float (double-precision)"))
  (return (`/Game/Main_Game/Logic/CurrencySystem/BPC_CurrencySystem.Currency` (`self.BPC_CurrencySystem`))))

(fn `SubtractCurrency`
  (params (Amount :type "Float (double-precision)") (CancelDueToLack :type Boolean))
  (returns (NewCurrency :type "Float (double-precision)") (Success :type Boolean))
  (bind _bpc_currencysystem (`self.BPC_CurrencySystem`))
  (if (and CancelDueToLack (> Amount (`/Game/Main_Game/Logic/CurrencySystem/BPC_CurrencySystem.Currency` _bpc_currencysystem)))
    (return (`/Game/Main_Game/Logic/CurrencySystem/BPC_CurrencySystem.Currency` (`self.BPC_CurrencySystem`)) false)
    (else
      (bind _newcurrency (`/Game/Main_Game/Logic/CurrencySystem/BPC_CurrencySystem.SubtractCurrency` _bpc_currencysystem Amount))
      (return _newcurrency true))))

(fn `TakeDamage`
  (params (DamageInfo :type "/Game/Main_Game/Logic/DamageSystem/S_DamageInfo Structure"))
  (returns (NewParam :type Boolean))
  (`/Game/Main_Game/Logic/DamageSystem/BPC_DamageSystem.TakeDamage` (`self.BPC_DamageSystem`) DamageInfo)
  (return false))

(fn `UserConstructionScript`
  (add `/Game/Main_Game/Logic/DamageSystem/BPC_DamageSystem.OnDeath` (`self.BPC_DamageSystem`) (`|CreateDelegate` :!event `Death`)))