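; BP_InstructorCharacter is an instructor character that opens a shop UI when the player walks into its box collision.
; On begin overlap it creates the WB_Shop widget once, or re-shows the cached one, and switches the player's input mode.
; On end overlap it only collapses the widget, leaving the input mode unchanged.
; An unconnected camera view-target blend call never runs.
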(event `self.BoxCollision.OnComponentBeginOverlap`
  (params (OverlappedComponent :type "PrimitiveComponent Object Reference") (OtherActor :type "Actor Object Reference") (OtherComp :type "PrimitiveComponent Object Reference") (OtherBodyIndex :type Integer) (bFromSweep :type Boolean) (SweepResult :type "HitResult Structure (by ref)"))
  (if (== OtherActor (`GameplayStatics.GetPlayerCharacter` 0))
    (bind _wb_shop (`self.WB_Shop`)
      (:`then`
        (set `Widget.Visibility` "Visible" _wb_shop)
        (`/Game/Main_Game/Logic/FunctionLibraries/BFL_UI_Utils.Set_InputMode` "NewEnumerator1" (`GameplayStatics.GetPlayerController` 0) true))
      (:`else`
        (bind _returnvalue (`|CreateWidget` "/Game/Main_Game/UI/Blueprints/WB_Shop.WB_Shop_C"))
        (bind _output_get (set `self.WB_Shop` _returnvalue))
        (`UserWidget.AddToViewport` _output_get 0)
        (`/Game/Main_Game/Logic/FunctionLibraries/BFL_UI_Utils.Set_InputMode` "NewEnumerator1" (`GameplayStatics.GetPlayerController` 0) true)))))

(event `self.BoxCollision.OnComponentEndOverlap`
  (params (OverlappedComponent :type "PrimitiveComponent Object Reference") (OtherActor :type "Actor Object Reference") (OtherComp :type "PrimitiveComponent Object Reference") (OtherBodyIndex :type Integer))
  (if (== OtherActor (`GameplayStatics.GetPlayerCharacter` 0))
    (set `Widget.Visibility` "Collapsed" (`self.WB_Shop`))))

(fn `UserConstructionScript`)