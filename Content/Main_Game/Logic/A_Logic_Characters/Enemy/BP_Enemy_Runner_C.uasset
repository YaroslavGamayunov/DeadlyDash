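; Runner enemy Blueprint that extends a parent enemy class with a projectile attack.
; On BeginPlay it adds its static mesh component to the Target array after running the parent logic.
; Attack runs the parent attack, spawns a Runner projectile just ahead of the actor along its forward vector, then signals attack end after a short delay.
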(event `self.ReceiveBeginPlay`
  (`parent.ReceiveBeginPlay`)
  (`KismetArrayLibrary.Array_Add` (`self.Target`) (`self.StaticMesh_0`)))

(event `self.Attack`
  (bind _returnvalue (`self.GetActorForwardVector`))
  (`parent.Attack`)
  (`|SpawnActorFromClass` "/Game/Main_Game/Logic/A_Logic_Characters/Projectiles/BP_Projectile_Runner.BP_Projectile_Runner_C" (`KismetMathLibrary.MakeTransform` (+ (`self.K2_GetActorLocation`) (* _returnvalue 100.0)) (`KismetMathLibrary.Conv_VectorToRotator` _returnvalue)) "AlwaysSpawn" "MultiplyWithRoot" null 250.0 null)
  (`KismetSystemLibrary.Delay` 0.2)
  (`self.OnAttackEnd`))

(fn `UserConstructionScript`
  (`parent.UserConstructionScript`))