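; BP_EnemyPawn_P is an enemy pawn, apparently a parent class, that supports interaction and focus highlighting.
; Interact fires an interact event and reports success.
; The focus toggle sets Render Custom Depth on each valid element of the Target array, then fires mouse enter or leave events.
; The interact and mouse events are empty here, and BeginPlay, overlap and Tick are unused.
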(event `Interact_Event`)

(event `EventOnMouseEnter`)

(event `EventOnMouseLeave`)

(fn `Interact`
  (returns (Success :type Boolean))
  (`self.Interact_Event`)
  (return true))

(fn `Interact_ToggleFocus_T`
  (params (Focus :type Boolean))
  (returns (SubjectToAbility :type Boolean))
  (for _array_element (`self.Target`)
    (`/Engine/EditorBlueprintResources/StandardMacros.IsValid` _array_element
      (:`Is Valid`
        (`PrimitiveComponent.SetRenderCustomDepth` _array_element Focus))))
  (if Focus
    (`self.EventOnMouseEnter`)
    (else
      (`self.EventOnMouseLeave`)))
  (return true))

(fn `UserConstructionScript`)