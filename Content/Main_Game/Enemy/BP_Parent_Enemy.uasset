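; BP_Parent_Enemy is a base enemy that hurts the player on contact and dies from any damage.
; BeginPlay caches a reference to the player character.
; Its Sphere overlap applies damage to any overlapping BP_PlayerCharacter.
; AnyDamage ignores the amount, prints a debug message, spawns an explosion emitter at the enemy's location and destroys the actor.
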(event `self.ReceiveBeginPlay`
  (bind _asbp_player_character (cast `/Game/Main_Game/Character/BP_PlayerCharacter` (`GameplayStatics.GetPlayerCharacter` 0)))
  (set `self.As BP Player Character` _asbp_player_character))

(event `self.Sphere.OnComponentBeginOverlap`
  (params (OverlappedComponent :type "PrimitiveComponent Object Reference") (OtherActor :type "Actor Object Reference") (OtherComp :type "PrimitiveComponent Object Reference") (OtherBodyIndex :type Integer) (bFromSweep :type Boolean) (SweepResult :type "HitResult Structure (by ref)"))
  (bind _asbp_player_character (cast `/Game/Main_Game/Character/BP_PlayerCharacter` OtherActor))
  (`GameplayStatics.ApplyDamage` _asbp_player_character 1.0))

(event `self.ReceiveAnyDamage`
  (params (Damage :type "Float (single-precision)") (DamageType :type "DamageType Object Reference") (InstigatedBy :type "Controller Object Reference") (DamageCauser :type "Actor Object Reference"))
  (`KismetSystemLibrary.PrintString` "enemy dead")
  (`GameplayStatics.SpawnEmitterAtLocation` "/Game/Starter/StarterContent/Particles/P_Explosion.P_Explosion" (`self.K2_GetActorLocation`))
  (`self.K2_DestroyActor`))

(fn `UserConstructionScript`)