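; BP_C_TurretWireSpline is a spline-driven wire, by its name for enemy turrets, with no runtime logic of its own.
; The construction script splits the spline into sections sized by the actor's X scale and adds an X-forward spline mesh for each, including one for the tail.
; A helper supplies each section's local endpoints and tangents, clamping tangent length to the section length so segments bend cleanly.
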(event `self.ReceiveBeginPlay`
  (`parent.ReceiveBeginPlay`))

(fn `Get Position and Tangent`
  (params (`Loop Index` :type Integer))
  (returns (Location :type "Vector Structure") (Tangent :type "Vector Structure"))
  (bind _spline (`self.Spline`))
  (bind _returnvalue (* `Loop Index` (`self.SectionLength`)))
  (return (`SplineComponent.GetLocationAtDistanceAlongSpline` _spline _returnvalue "Local") (`KismetMathLibrary.ClampVectorSize` (`SplineComponent.GetTangentAtDistanceAlongSpline` _spline _returnvalue "Local") 0.0 (`self.SectionLength`))))

(fn `UserConstructionScript`
  (bind _returnvalue_x (`KismetMathLibrary.BreakVector` (`self.GetActorScale3D`)))
  (`parent.UserConstructionScript`)
  (set `self.SectionLength` (* _returnvalue_x 100.0))
  (bind _output_get (set `self.NumberOfSections` (`KismetMathLibrary.FTrunc` (/ (`SplineComponent.GetSplineLength` (`self.Spline`)) (`self.SectionLength`)))))
  (for _index (range (+ _output_get 1))
    (set `self.LoopIndex` _index)
    (bind _returnvalue (`AddComponent|NODE_AddSplineMeshComponent-0`))
    (`SplineMeshComponent.SetForwardAxis` _returnvalue "X" true)
    (bind (_location _tangent) (`self.Get Position and Tangent` (`self.LoopIndex`)))
    (bind (_location_2 _tangent_2) (`self.Get Position and Tangent` (+ (`self.LoopIndex`) 1)))
    (`SplineMeshComponent.SetStartAndEnd` _returnvalue _location _tangent _location_2 _tangent_2 true)))