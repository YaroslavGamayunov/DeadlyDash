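; BP_BaseEnemy is a base enemy pawn that moves toward the player.
; On BeginPlay it calls the parent event, then issues a single AI MoveTo targeting the first player character as an actor.
; Tick and the construction script add no logic.
; Disconnected leftover nodes hold unused experiments with SimpleMoveToLocation and visibility line traces to the player.
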(event `self.ReceiveBeginPlay`
  (`parent.ReceiveBeginPlay`)
  (`|AIMoveTo` self (0.0 0.0 0.0) (`GameplayStatics.GetPlayerCharacter` 0)))

(event `self.ReceiveTick`
  (params (DeltaSeconds :type "Float (single-precision)")))

(fn `UserConstructionScript`
  (`parent.UserConstructionScript`))