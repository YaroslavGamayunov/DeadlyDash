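; BP_DashSpawner scatters four BP_DashTrigger actors, each yawed a further 90 degrees, around the player shortly after play begins.
; It picks random reachable navmesh points near the player, retrying any that project outside hardcoded 1920x1080 screen margins or overlap objects in a sphere trace.
; The Reset event destroys all existing triggers and spawns a fresh set.
; Timer-related events are empty or unconnected.
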(event `self.ReceiveBeginPlay`
  (bind _asbp_player_character (cast `/Game/Main_Game/Character/BP_PlayerCharacter` (`GameplayStatics.GetPlayerCharacter` 0)))
  (bind _output_get (set `self.As BP Player Character` _asbp_player_character))
  (`KismetSystemLibrary.Delay` 1.0)
  (for _index (range 4) :!label _label
    (bind _output_get_2 (set `self.Random Location` (`NavigationSystemV1.K2_GetRandomReachablePointInRadius` (`self.K2_GetActorLocation` _output_get) 1100.0 null null) :!label _label_2))
    (bind (_x _y) (`KismetMathLibrary.BreakVector2D` (`WidgetLayoutLibrary.ProjectWorldLocationToWidgetPosition` (`GameplayStatics.GetPlayerController` 0) _output_get_2 true)))
    (if (or (< _x 70.0) (> _x 1850.0) (< _y 70.0) (> _y 1010.0))
      (`self.CustomEvent`)
      (else
        (bind (_outhits _returnvalue) (`KismetSystemLibrary.SphereTraceMultiForObjects` :`Start` _output_get_2 :`End` _output_get_2 :`Radius` 100.0 :`ObjectTypes` (`|MakeArray` "ObjectTypeQuery2" "ObjectTypeQuery3" "ObjectTypeQuery7" :!type "EObjectTypeQuery Enum") :`DrawDebugType` "ForDuration"))
        (if _returnvalue
          (`self.CustomEvent`)
          (else
            (`|SpawnActorFromClass` "/Game/Main_Game/A_Logic/BP_DashTrigger.BP_DashTrigger_C" (`KismetMathLibrary.MakeTransform` (`self.Random Location`) (`KismetMathLibrary.MakeRotator` 0.0 0.0 (`KismetMathLibrary.Conv_IntToDouble` (* _index 90)))) "AlwaysSpawn" "MultiplyWithRoot" null null)))))))

(event `Reset`
  (bind _outactors (`GameplayStatics.GetAllActorsOfClass` "/Game/Main_Game/A_Logic/BP_DashTrigger.BP_DashTrigger_C"))
  (for _array_element _outactors
    (`self.K2_DestroyActor` _array_element))
  (goto _label))

(event `CustomEvent`
  (goto _label_2))

(event `Spawn Timer`)

(event `DashSpawn`)

(fn `UserConstructionScript`)